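; BP_StandVente is a sales stand actor where an article and a price are selected through a WB_StandInterface widget component.
; Overlap of its box by ThirdPersonCharacter looks up the selected article in the ListArticle map.
; Enter stores the chosen price and repeats that lookup.
; VerifPrix prints whether the price is above, below or equal to the article's optimal price, but its call is unwired.
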(event OnComponentBeginOverlap(Box)
  (params (OverlappedComponent :type Primitive%20Component%20Object%20Reference) (OtherActor :type Actor%20Object%20Reference) (OtherComp :type Primitive%20Component%20Object%20Reference) (OtherBodyIndex :type Integer) (bFromSweep :type Boolean) (SweepResult :type Hit%20Result%20Structure%20%28by%20ref%29))
  (bind _ascharacter (Utilities|Casting|CastToCharacter OtherActor))
  (Utilities|Casting|CastToThirdPersonCharacter _ascharacter)
  (CallFunction|ChooseItem))

(event Custom|VerifPrix
  (bind _articleon (Variables|Default|GetArticleOn))
  ;[1 1 1] Verif Prix
  (if (> (Variables|Default|GetPrixChoisi) (Variables|/Game/BP_Article.BP_Article_C|GetPrixOptimal _articleon))
    (Development|PrintString "Trop")
    (elif (< (Variables|Default|GetPrixChoisi) (Variables|/Game/BP_Article.BP_Article_C|GetPrixOptimal _articleon))
      (Development|PrintString "Moins")
      (elif (== (Variables|Default|GetPrixChoisi) (Variables|/Game/BP_Article.BP_Article_C|GetPrixOptimal _articleon))
        (Development|PrintString "Egal")))))

(event Custom|ChooseItem
  (params (En%20Vente :type S%20Article%20Structure))
  ;[1 1 1] Choose Item
  (Variables|Default|SetArticleOn (.Value (Utilities|Map|Find (Variables|Default|GetListArticle) (Variables|/Game/WB_StandInterface.WB_StandInterface_C|GetArticleSelected (Variables|Default|GetAs%20WB%20Stand%20Interface))))))

(event Custom|SetPrix
  ;[1 1 1] Set Prix
  (Variables|Default|SetPrixChoisi (Variables|/Game/WB_StandInterface.WB_StandInterface_C|GetPrixSelected (Variables|Default|GetAs%20WB%20Stand%20Interface))))

(event EventBeginPlay
  (bind _aswb_stand_interface (Utilities|Casting|CastToWB_StandInterface (UserInterface|GetWidget (Variables|Default|GetWidget))))
  (Variables|Default|SetAs%20WB%20Stand%20Interface _aswb_stand_interface))

(event Collision|EventActorBeginOverlap
  (params (OtherActor :type Actor%20Object%20Reference)))

(event EventTick
  (params (DeltaSeconds :type Float%20%28single-precision%29)))

(event Input|KeyboardEvents|Enter
  (params (Key :type Key%20Structure :default "None"))
  (:Pressed
    (CallFunction|SetPrix)
    (CallFunction|ChooseItem)))

(fn ConstructionScript)